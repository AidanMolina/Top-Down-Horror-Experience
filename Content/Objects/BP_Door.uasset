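; Lockable sliding door that opens when the player has the required inventory item.
; Actor overlap registers it as the player's current door and, once unlocked, slides it between StartPoint and EndPoint; sphere overlap shows a widget while locked.
; Unlock matches inventory names against Unlocker, or MessageUnlocker as fallback, consuming the match and opening the door.
; The failure message fires for every non-matching item, as the loop never breaks.
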(event OnComponentBeginOverlap(Sphere)
  (params (OverlappedComponent :type Primitive%20Component%20Object%20Reference) (OtherActor :type Actor%20Object%20Reference) (OtherComp :type Primitive%20Component%20Object%20Reference) (OtherBodyIndex :type Integer) (bFromSweep :type Boolean) (SweepResult :type Hit%20Result%20Structure%20%28by%20ref%29))
  (if (not (Variables|Default|GetIsUnlocked))
    (Development|SetHiddeninGame (Variables|Default|GetWidget) false false)))

(event OnComponentEndOverlap(Sphere)
  (params (OverlappedComponent :type Primitive%20Component%20Object%20Reference) (OtherActor :type Actor%20Object%20Reference) (OtherComp :type Primitive%20Component%20Object%20Reference) (OtherBodyIndex :type Integer))
  (Development|SetHiddeninGame (Variables|Default|GetWidget) true false))

(event Custom|JustUnlocked
  (Components|MoveComponentTo (Variables|Default|GetDoor) (Variables|/Script/Engine.SceneComponent|GetRelativeLocation (Variables|Default|GetEnd%20Point)) "0, 0, 0" false false 0.5 false))

(event Custom|Unlock
  (bind _asplayer_character (Utilities|Casting|CastToPlayerCharacter (Game|Player|GetPlayerPawn 0)))
  (if (Utilities|IsValid (Variables|Default|GetUnlocker))
    (for _array_element (Variables|/Script/MyProject.InventoryComponent|GetItems (Variables|/Script/MyProject.PlayerCharacter|GetInventory _asplayer_character))
      (if (Utilities|Enum|Equal(Enum) (Variables|/Script/MyProject.InteractableObjects|GetItemName _array_element) (Variables|/Script/MyProject.InteractableObjects|GetItemName (Variables|Default|GetUnlocker)))
        (Variables|Default|SetIsUnlocked true)
        (CallFunction|JustUnlocked)
        (bind _asbp_my_player_character (Utilities|Casting|CastToBP_MyPlayerCharacter (Game|Player|GetPlayerPawn 0)))
        (Default|UsedDoor _asbp_my_player_character (Utilities|Text|FormatText "Used {item} to unlock the door." (Variables|/Script/MyProject.InteractableObjects|GetItemName _array_element)))
        (Class|InventoryComponent|RemoveItem (Variables|/Script/MyProject.PlayerCharacter|GetInventory _asplayer_character) _array_element)
        (else
          (bind _asbp_my_player_character_2 (Utilities|Casting|CastToBP_MyPlayerCharacter (Game|Player|GetPlayerPawn 0)))
          (Default|UsedDoor _asbp_my_player_character_2 (Utilities|Text|FormatText "You do not have the right item to unlock this door.")))))
    (elif (Utilities|IsValid (Variables|Default|GetMessageUnlocker))
      (for _array_element_2 (Variables|/Script/MyProject.InventoryComponent|GetItems (Variables|/Script/MyProject.PlayerCharacter|GetInventory _asplayer_character))
        (if (Utilities|Enum|Equal(Enum) (Variables|/Script/MyProject.InteractableObjects|GetItemName _array_element_2) (Variables|/Script/MyProject.InteractableObjects|GetItemName (Variables|Default|GetMessageUnlocker)))
          (Variables|Default|SetIsUnlocked true)
          (CallFunction|JustUnlocked)
          (bind _asbp_my_player_character_3 (Utilities|Casting|CastToBP_MyPlayerCharacter (Game|Player|GetPlayerPawn 0)))
          (Default|UsedDoor _asbp_my_player_character_3 (Utilities|Text|FormatText "Used {item} to unlock the door." (Variables|/Script/MyProject.InteractableObjects|GetItemName _array_element)))
          (Class|InventoryComponent|RemoveItem (Variables|/Script/MyProject.PlayerCharacter|GetInventory _asplayer_character) _array_element)
          (else
            (bind _asbp_my_player_character_4 (Utilities|Casting|CastToBP_MyPlayerCharacter (Game|Player|GetPlayerPawn 0)))
            (Default|UsedDoor _asbp_my_player_character_4 (Utilities|Text|FormatText "You do not have the right item to unlock this door."))))))))

(event Custom|OnActorBeginOverlapping
  (params (OverlappedActor :type Actor%20Object%20Reference) (OtherActor :type Actor%20Object%20Reference))
  (Variables|Default|SetIsNear true)
  (bind _asbp_my_player_character (Utilities|Casting|CastToBP_MyPlayerCharacter (Game|GetPlayerCharacter 0)))
  (Default|SetCurrentDoor _asbp_my_player_character self)
  (Development|PrintString "Is Near is True")
  (if (Variables|Default|GetIsUnlocked)
    (Components|MoveComponentTo (Variables|Default|GetDoor) (Variables|/Script/Engine.SceneComponent|GetRelativeLocation (Variables|Default|GetEnd%20Point)) "0, 0, 0" false false 0.5 false)))

(event Custom|OnActorEndOverlapping
  (params (OverlappedActor :type Actor%20Object%20Reference) (OtherActor :type Actor%20Object%20Reference))
  (Variables|Default|SetIsNear false)
  (Development|PrintString "Is Near is False")
  (if (Variables|Default|GetIsUnlocked)
    (Components|MoveComponentTo (Variables|Default|GetDoor) (Variables|/Script/Engine.SceneComponent|GetRelativeLocation (Variables|Default|GetStart%20Point)) "0, 0, 0" false false 0.5 false)))

(event EventBeginPlay
  (bind _door (Variables|Default|GetDoor))
  (bind _returnvalue (Components|GetOwner _door))
  (bind _returnvalue_2 (Actor|GetComponentbyClass _returnvalue "/Script/Engine.StaticMeshComponent"))
  (Utilities|IsValid _returnvalue_2
    (:Is%20Valid
      (Variables|Default|SetStatic%20Mesh%20Ref _returnvalue_2)
      (Collision|BindEventtoOnActorBeginOverlap _returnvalue (delegate Custom|OnActorBeginOverlapping))
      (Collision|BindEventtoOnActorEndOverlap _returnvalue (delegate Custom|OnActorEndOverlapping)))))

(fn ConstructionScript)