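; BP_InventoryObjects is an inventory object that signals proximity with an outline-ready highlight and a widget, with no pickup logic.
; BeginPlay caches the owner's static mesh and binds actor overlap events that toggle its Custom Depth rendering and an IsNear flag, with debug prints.
; The Box component's own overlaps separately show and hide the widget.
; Neither overlap path filters which actor triggers it.
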(event OnComponentBeginOverlap(Box)
  (params (OverlappedComponent :type Primitive%20Component%20Object%20Reference) (OtherActor :type Actor%20Object%20Reference) (OtherComp :type Primitive%20Component%20Object%20Reference) (OtherBodyIndex :type Integer) (bFromSweep :type Boolean) (SweepResult :type Hit%20Result%20Structure%20%28by%20ref%29))
  (Development|SetHiddeninGame (Variables|Default|GetWidget) false false))

(event OnComponentEndOverlap(Box)
  (params (OverlappedComponent :type Primitive%20Component%20Object%20Reference) (OtherActor :type Actor%20Object%20Reference) (OtherComp :type Primitive%20Component%20Object%20Reference) (OtherBodyIndex :type Integer))
  (Development|SetHiddeninGame (Variables|Default|GetWidget) true false))

(event Custom|OnActorBeginOverlapping
  (params (OverlappedActor :type Actor%20Object%20Reference) (OtherActor :type Actor%20Object%20Reference))
  (Rendering|SetRenderCustomDepth (Variables|Default|GetStaticMeshRef) true)
  (Variables|Default|SetIsNear true)
  (Development|PrintString "Is Near is True"))

(event Custom|OnActorEndOverlapping
  (params (OverlappedActor :type Actor%20Object%20Reference) (OtherActor :type Actor%20Object%20Reference))
  (Rendering|SetRenderCustomDepth (Variables|Default|GetStaticMeshRef) false)
  (Variables|Default|SetIsNear false)
  (Development|PrintString "Is Near is False"))

(event EventBeginPlay
  (bind _cube (Variables|Default|GetCube))
  (bind _returnvalue (Components|GetOwner _cube))
  (bind _returnvalue_2 (Actor|GetComponentbyClass _returnvalue "/Script/Engine.StaticMeshComponent"))
  (Utilities|IsValid _returnvalue_2
    (:Is%20Valid
      (Variables|Default|SetStaticMeshRef _returnvalue_2)
      (Collision|BindEventtoOnActorBeginOverlap _returnvalue (delegate Custom|OnActorBeginOverlapping))
      (Collision|BindEventtoOnActorEndOverlap _returnvalue (delegate Custom|OnActorEndOverlapping)))))

(fn ConstructionScript)