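; BP_DoubleDoors is a two-panel sliding door that opens when overlapped while unlocked and closes when the overlap ends.
; Begin overlap sets IsNear and registers the door with the player character via SetCurrentDoor, without checking which actor overlapped.
; MoveComponentTo slides Door to EndPoint and Door1 to EndPoint1, with paired events driving Door1; both return to the shared StartPoint.
; A JustUnlocked opening path exists but never runs.
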(event Custom|Other%20Door%20Open
  (bind _door1 (Variables|Default|GetDoor1))
  (Components|MoveComponentTo _door1 (Variables|/Script/Engine.SceneComponent|GetRelativeLocation (Variables|Default|GetEnd%20Point1)) (Variables|/Script/Engine.SceneComponent|GetRelativeRotation _door1) false false 0.5 false))

(event Custom|Other%20Door%20Close
  (bind _door1 (Variables|Default|GetDoor1))
  (Components|MoveComponentTo _door1 (Variables|/Script/Engine.SceneComponent|GetRelativeLocation (Variables|Default|GetStart%20Point)) (Variables|/Script/Engine.SceneComponent|GetRelativeRotation _door1) false false 0.5 false))

(event EventBeginPlay
  (|CallParentFunction) ; This node is disabled and will not be called.\nDrag off pins to build functionality.
)

(event EventOnActorBeginOverlapping
  (params (OverlappedActor :type Actor%20Object%20Reference) (OtherActor :type Actor%20Object%20Reference))
  (Variables|Default|SetIsNear true)
  (bind _asbp_my_player_character (Utilities|Casting|CastToBP_MyPlayerCharacter (Game|GetPlayerCharacter 0)))
  (Default|SetCurrentDoor _asbp_my_player_character self)
  (Development|PrintString "Is Near is True")
  (if (Variables|Default|GetIsUnlocked)
    (CallFunction|OtherDoorOpen)
    (Components|MoveComponentTo (Variables|Default|GetDoor) (Variables|/Script/Engine.SceneComponent|GetRelativeLocation (Variables|Default|GetEnd%20Point)) "0, 0, 0" false false 0.5 false)))

(event EventOnActorEndOverlapping
  (params (OverlappedActor :type Actor%20Object%20Reference) (OtherActor :type Actor%20Object%20Reference))
  (Variables|Default|SetIsNear false)
  (Development|PrintString "Is Near is False")
  (if (Variables|Default|GetIsUnlocked)
    (CallFunction|OtherDoorClose)
    (Components|MoveComponentTo (Variables|Default|GetDoor) (Variables|/Script/Engine.SceneComponent|GetRelativeLocation (Variables|Default|GetStart%20Point)) "0, 0, 0" false false 0.5 false)))

(fn ConstructionScript
  (|CallParentFunction))