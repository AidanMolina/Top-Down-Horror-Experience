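; BP_GunObject is a world rifle object that highlights when approached and shows the ammo HUD when used.
; Actor overlaps toggle the mesh's custom depth and an IsNear flag, while Box overlaps show or hide a prompt widget.
; OnUse creates and refreshes AmmoWidget, then clears the highlight and prompt.
; It moves the actor below the world origin instead of destroying it.
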(event OnComponentBeginOverlap(Box)
  (params (OverlappedComponent :type Primitive%20Component%20Object%20Reference) (OtherActor :type Actor%20Object%20Reference) (OtherComp :type Primitive%20Component%20Object%20Reference) (OtherBodyIndex :type Integer) (bFromSweep :type Boolean) (SweepResult :type Hit%20Result%20Structure%20%28by%20ref%29))
  (Utilities|Casting|CastToBP_MyPlayerCharacter OtherActor)
  (Development|SetHiddeninGame (Variables|Default|GetWidget) false false))

(event OnComponentEndOverlap(Box)
  (params (OverlappedComponent :type Primitive%20Component%20Object%20Reference) (OtherActor :type Actor%20Object%20Reference) (OtherComp :type Primitive%20Component%20Object%20Reference) (OtherBodyIndex :type Integer))
  (Development|SetHiddeninGame (Variables|Default|GetWidget) true false))

(event Custom|OnActorBeginOverlapping
  (params (OverlappedActor :type Actor%20Object%20Reference) (OtherActor :type Actor%20Object%20Reference))
  (Utilities|Casting|CastToBP_MyPlayerCharacter OtherActor)
  (Rendering|SetRenderCustomDepth (Variables|Default|GetStaticMeshRef) true)
  (Variables|Default|SetIsNear true))

(event Custom|OnActorEndOverlapping
  (params (OverlappedActor :type Actor%20Object%20Reference) (OtherActor :type Actor%20Object%20Reference))
  (Rendering|SetRenderCustomDepth (Variables|Default|GetStaticMeshRef) false)
  (Variables|Default|SetIsNear false))

(event Collision|EventActorBeginOverlap
  (params (OtherActor :type Actor%20Object%20Reference)))

(event EventTick
  (params (DeltaSeconds :type Float%20%28single-precision%29)))

(event EventOnUse
  (params (Character :type Player%20Character%20Object%20Reference))
  (bind _returnvalue (UserInterface|CreateWidget "/Game/Objects/AmmoWidget.AmmoWidget_C" (Game|GetPlayerController 0)))
  (UserInterface|Viewport|AddtoViewport _returnvalue 0)
  (Default|RefreshUI _returnvalue)
  (Transformation|SetActorLocation "0.000000,0.000000,-500.000000" false false)
  (Variables|Default|SetIsNear false)
  (Rendering|SetRenderCustomDepth (Variables|Default|GetStaticMeshRef) false)
  (Development|SetHiddeninGame (Variables|Default|GetWidget) true false))

(event EventBeginPlay
  (bind _rifle (Variables|Default|GetRifle))
  (bind _returnvalue (Components|GetOwner _rifle))
  (bind _returnvalue_2 (Actor|GetComponentbyClass _returnvalue "/Script/Engine.StaticMeshComponent"))
  (Utilities|IsValid _returnvalue_2
    (:Is%20Valid
      (Variables|Default|SetStaticMeshRef _returnvalue_2)
      (Collision|BindEventtoOnActorBeginOverlap _returnvalue (delegate Custom|OnActorBeginOverlapping))
      (Collision|BindEventtoOnActorEndOverlap _returnvalue (delegate Custom|OnActorEndOverlapping)))))

(fn ConstructionScript)