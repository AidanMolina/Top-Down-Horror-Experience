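; BP_MysteriousDoor is a door that unlocks once the player has collected three specific items.
; Its Unlock event scans the player character's inventory, matching item names against Object1, Object2 and Object3 and setting a flag for each.
; After each match it calls JustUnlocked if all three flags are true.
; The flags are cleared only on BeginPlay, so they persist between unlock attempts.
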(event EventBeginPlay
  (|CallParentFunction)
  (Variables|Default|SetHasObject1 false)
  (Variables|Default|SetHasObject2 false)
  (Variables|Default|SetHasObject3 false))

(event Collision|EventActorBeginOverlap
  (params (OtherActor :type Actor%20Object%20Reference)))

(event EventTick
  (params (DeltaSeconds :type Float%20%28single-precision%29)))

(event EventUnlock
  (bind _asplayer_character (Utilities|Casting|CastToPlayerCharacter (Game|Player|GetPlayerPawn 0)))
  (for _array_element (Variables|/Script/MyProject.InventoryComponent|GetItems (Variables|/Script/MyProject.PlayerCharacter|GetInventory _asplayer_character))
    (if (Utilities|Enum|Equal(Enum) (Variables|/Script/MyProject.InteractableObjects|GetItemName _array_element) (Variables|/Script/MyProject.InteractableObjects|GetItemName (Variables|Default|GetObject1)))
      (Variables|Default|SetHasObject1 true)
      (if (Math|Boolean|ANDBoolean (Variables|Default|GetHasObject1) (Variables|Default|GetHasObject2) (Variables|Default|GetHasObject3)) :!label _label
        (CallFunction|JustUnlocked))
      (elif (Utilities|Enum|Equal(Enum) (Variables|/Script/MyProject.InteractableObjects|GetItemName _array_element) (Variables|/Script/MyProject.InteractableObjects|GetItemName (Variables|Default|GetObject2)))
        (Variables|Default|SetHasObject2 true)
        (goto _label)
        (elif (Utilities|Enum|Equal(Enum) (Variables|/Script/MyProject.InteractableObjects|GetItemName _array_element) (Variables|/Script/MyProject.InteractableObjects|GetItemName (Variables|Default|GetObject3)))
          (Variables|Default|SetHasObject3 true)
          (goto _label))))))

(fn ConstructionScript
  (|CallParentFunction))