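; BP_EscapePod is an escape pod actor that serves as the game's exit to the credits.
; Actor overlaps track proximity in IsNear and register the pod on BP_MyPlayerCharacter, while a separate Box trigger shows and hides a widget.
; EndGame, which nothing here calls, switches to UI-only input with a cursor and loads the credits as a level instance rather than opening the level.
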(event OnComponentBeginOverlap(Box)
  (params (OverlappedComponent :type Primitive%20Component%20Object%20Reference) (OtherActor :type Actor%20Object%20Reference) (OtherComp :type Primitive%20Component%20Object%20Reference) (OtherBodyIndex :type Integer) (bFromSweep :type Boolean) (SweepResult :type Hit%20Result%20Structure%20%28by%20ref%29))
  (Development|SetHiddeninGame (Variables|Default|GetWidget) false false))

(event OnComponentEndOverlap(Box)
  (params (OverlappedComponent :type Primitive%20Component%20Object%20Reference) (OtherActor :type Actor%20Object%20Reference) (OtherComp :type Primitive%20Component%20Object%20Reference) (OtherBodyIndex :type Integer))
  (Development|SetHiddeninGame (Variables|Default|GetWidget) true false))

(event Custom|EndGame
  (bind _returnvalue (Game|GetPlayerController 0))
  (Variables|/Script/Engine.PlayerController|SetbShowMouseCursor _returnvalue true)
  (Input|SetInputModeUIOnly _returnvalue 0 "DoNotLock" false)
  (Class|LevelStreamingDynamic|LoadLevelInstancebySoftObjectPtr "/Game/Maps/CreditsLevel.CreditsLevel" "0, 0, 0" "0, 0, 0" "" 0 false))

(event Custom|OnActorBeginOverlapping
  (params (OverlappedActor :type Actor%20Object%20Reference) (OtherActor :type Actor%20Object%20Reference))
  (bind _asbp_my_player_character (Utilities|Casting|CastToBP_MyPlayerCharacter OtherActor))
  (Variables|/Game/Character/BP_MyPlayerCharacter.BP_MyPlayerCharacter_C|SetEscapePod _asbp_my_player_character self)
  (Variables|Default|SetIsNear true)
  (Development|PrintString "Is Near is True"))

(event Custom|OnActorEndOverlapping
  (params (OverlappedActor :type Actor%20Object%20Reference) (OtherActor :type Actor%20Object%20Reference))
  (Variables|Default|SetIsNear false)
  (Development|PrintString "Is Near is False"))

(event EventBeginPlay
  (bind _pod (Variables|Default|GetPod))
  (bind _returnvalue (Components|GetOwner _pod))
  (bind _returnvalue_2 (Actor|GetComponentbyClass _returnvalue "/Script/Engine.StaticMeshComponent"))
  (Utilities|IsValid _returnvalue_2
    (:Is%20Valid
      (Variables|Default|SetStaticMeshRef _returnvalue_2)
      (Collision|BindEventtoOnActorBeginOverlap _returnvalue (delegate Custom|OnActorBeginOverlapping))
      (Collision|BindEventtoOnActorEndOverlap _returnvalue (delegate Custom|OnActorEndOverlapping)))))

(fn ConstructionScript)