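; Mysterious sphere object that vanishes from view when used.
; OnUse moves the actor to a fixed location below the world origin instead of destroying it.
; It also clears the IsNear flag, turns off custom depth rendering on the mesh and hides the widget.
; BeginPlay, overlap and Tick are disabled stubs, and the construction script only calls the parent.
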(event EventBeginPlay
  (|CallParentFunction) ; This node is disabled and will not be called.\nDrag off pins to build functionality.
)

(event Collision|EventActorBeginOverlap
  (params (OtherActor :type Actor%20Object%20Reference)))

(event EventTick
  (params (DeltaSeconds :type Float%20%28single-precision%29)))

(event EventOnUse
  (params (Character :type Player%20Character%20Object%20Reference))
  (Transformation|SetActorLocation "0.000000,0.000000,-500.000000" false false)
  (Variables|Default|SetIsNear false)
  (Rendering|SetRenderCustomDepth (Variables|Default|GetStaticMeshRef) false)
  (Development|SetHiddeninGame (Variables|Default|GetWidget) true false)
  (Development|SetHiddeninGame (Variables|Default|GetWidget) true false))

(fn ConstructionScript
  (|CallParentFunction))