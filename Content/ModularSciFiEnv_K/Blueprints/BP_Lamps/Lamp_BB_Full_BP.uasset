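; Placeable sci-fi environment lamp Blueprint that pairs a spotlight with a lamp mesh.
; The construction script applies the light radius, color and intensity variables to the SpotLight.
; It creates a dynamic instance of the mesh's second material slot and sets its D_EmissTint parameter to the same color, so the emissive tint matches the light.
; The event graph has no active logic.
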(event EventBeginPlay)

(event Collision|EventActorBeginOverlap
  (params (OtherActor :type Actor%20Object%20Reference)))

(event EventTick
  (params (DeltaSeconds :type Float%20%28single-precision%29)))

(fn ConstructionScript
  (bind _lightmesh (Variables|Default|GetLightMesh))
  (bind _spotlight (Variables|Default|GetSpotLight))
  (Rendering|Lighting|SetAttenuationRadius _spotlight (Variables|BP_Light|GetLightRadius))
  (Rendering|Components|Light|SetLightColor _spotlight (Variables|BP_Light|GetLightColor) true)
  (Rendering|Components|Light|SetIntensity _spotlight (Variables|BPLight|GetLightIntensity))
  (bind _returnvalue (Rendering|Material|CreateDynamicMaterialInstance _lightmesh 1 (Rendering|Material|GetMaterial _lightmesh 1) "LightMeshMaterial" :!class /Script/Engine.PrimitiveComponent))
  (bind _output_get (Variables|BPLight|SetLightMeshMaterialInstance _returnvalue))
  (Rendering|Material|SetVectorParameterValue _output_get "D_EmissTint" (Variables|BP_Light|GetLightColor) :!class /Script/Engine.MaterialInstanceDynamic))