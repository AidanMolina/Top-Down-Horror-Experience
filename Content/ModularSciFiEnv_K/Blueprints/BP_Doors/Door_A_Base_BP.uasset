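; Base sci-fi sliding double door that opens when the player pawn enters its trigger and closes when it leaves.
; A timeline at configurable speed slides DoorL and DoorR apart in opposite directions along local Y, scaled by OpenSize, and reverses to close.
; Overlaps during movement set pending open or close flags, which the timeline's Finished handler checks by direction to clear or run the queued action.
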(event OnComponentBeginOverlap(Trigger)
  (params (OverlappedComponent :type Primitive%20Component%20Object%20Reference) (OtherActor :type Actor%20Object%20Reference) (OtherComp :type Primitive%20Component%20Object%20Reference) (OtherBodyIndex :type Integer) (bFromSweep :type Boolean) (SweepResult :type Hit%20Result%20Structure%20%28by%20ref%29))
  (if (== OtherActor (Game|Player|GetPlayerPawn 0))
    (CallFunction|TryStartOpen)))

(event OnComponentEndOverlap(Trigger)
  (params (OverlappedComponent :type Primitive%20Component%20Object%20Reference) (OtherActor :type Actor%20Object%20Reference) (OtherComp :type Primitive%20Component%20Object%20Reference) (OtherBodyIndex :type Integer))
  (if (== (stale OnComponentBeginOverlap(Trigger) OtherActor) (Game|Player|GetPlayerPawn 0))
    (CallFunction|TryStartClose)))

(event Custom|TryStartClose
  (if (Variables|Default|GetIsMoving)
    (Variables|Default|SetIsNeedClose true)
    (else
      (CallFunction|StartClose))))

(event Custom|StartClose
  (Variables|Default|SetIsMoving true)
  (bind (_direction _opening) (Timeline|OpenDoor Reverse)
    (:Update
      (Transformation|SetRelativeLocation (Variables|Default|GetDoor_L) (Math|Vector|MakeVector 0.0 (* _opening (Variables|Default|GetOpenSize)) 0.0) false false)
      (Transformation|SetRelativeLocation (Variables|Default|GetDoor_R) (Math|Vector|MakeVector 0.0 (* (* _opening (Variables|Default|GetOpenSize)) -1.0) 0.0) false false))
    (:Finished
      (switch Utilities|FlowControl|Switch|SwitchonETimelineDirection _direction
        (:Forward
          (Variables|Default|SetIsMoving false)
          (if (Variables|Default|GetIsNeedOpen)
            (Variables|Default|SetIsNeedOpen false)
            (elif (Variables|Default|GetIsNeedClose)
              (CallFunction|TryStartClose))))
        (:Backward
          (Variables|Default|SetIsMoving false)
          (if (Variables|Default|GetIsNeedClose)
            (Variables|Default|SetIsNeedClose false)
            (elif (Variables|Default|GetIsNeedOpen)
              (CallFunction|TryStartOpen))))))))

(event Custom|TryStartOpen
  (if (Variables|Default|GetIsMoving)
    (Variables|Default|SetIsNeedOpen true)
    (else
      (CallFunction|StartOpen))))

(event Custom|StartOpen
  (Variables|Default|SetIsMoving true)
  (bind (_direction _opening) (Timeline|OpenDoor Play)
    (:Update
      (Transformation|SetRelativeLocation (Variables|Default|GetDoor_L) (Math|Vector|MakeVector 0.0 (* _opening (Variables|Default|GetOpenSize)) 0.0) false false)
      (Transformation|SetRelativeLocation (Variables|Default|GetDoor_R) (Math|Vector|MakeVector 0.0 (* (* _opening (Variables|Default|GetOpenSize)) -1.0) 0.0) false false))
    (:Finished
      (switch Utilities|FlowControl|Switch|SwitchonETimelineDirection _direction
        (:Forward
          (Variables|Default|SetIsMoving false)
          (if (Variables|Default|GetIsNeedOpen)
            (Variables|Default|SetIsNeedOpen false)
            (elif (Variables|Default|GetIsNeedClose)
              (CallFunction|TryStartClose))))
        (:Backward
          (Variables|Default|SetIsMoving false)
          (if (Variables|Default|GetIsNeedClose)
            (Variables|Default|SetIsNeedClose false)
            (elif (Variables|Default|GetIsNeedOpen)
              (CallFunction|TryStartOpen))))))))

(event EventBeginPlay
  (Components|Timeline|SetPlayRate (Variables|Default|GetOpenDoor) (Variables|Default|GetAnimSpeed)))

(fn ConstructionScript)