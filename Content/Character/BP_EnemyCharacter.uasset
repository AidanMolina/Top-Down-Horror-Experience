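; BP_EnemyCharacter is an enemy that chases the player character and calls Attack on reaching it.
; PawnSensing sight of a player starts an AI MoveTo toward them, while overlapping the Radius component also stores the player and starts a chase.
; Each sighting refreshes a retriggerable delay; when it expires, the enemy moves back to the ReturnParameters actor and adopts its rotation on arrival.
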(event OnSeePawn(PawnSensing)
  (params (Pawn :type Pawn%20Object%20Reference))
  (bind _self self)
  (if (Utilities|ClassIsChildOf (Utilities|GetClass Pawn) "/Game/Character/BP_MyPlayerCharacter.BP_MyPlayerCharacter_C")
    (Utilities|FlowControl|Sequence
      (:then_0
        (AI|AIMoveTo _self "0, 0, 0" Pawn 75.0 false
          (:OnSuccess
            (Class|EnemyCharacter|Attack))))
      (:then_1
        (Utilities|FlowControl|RetriggerableDelay 3.0)
        (AI|AIMoveTo _self "0, 0, 0" (Variables|Default|GetReturnParameters) 5.0 false
          (:OnSuccess
            (Transformation|SetActorRotation self (Transformation|GetActorRotation (Variables|Default|GetReturnParameters)))))))))

(event OnComponentBeginOverlap(Radius)
  (params (OverlappedComponent :type Primitive%20Component%20Object%20Reference) (OtherActor :type Actor%20Object%20Reference) (OtherComp :type Primitive%20Component%20Object%20Reference) (OtherBodyIndex :type Integer) (bFromSweep :type Boolean) (SweepResult :type Hit%20Result%20Structure%20%28by%20ref%29))
  (bind _asbp_my_player_character (Utilities|Casting|CastToBP_MyPlayerCharacter OtherActor))
  (bind _output_get (Variables|Default|SetPlayer _asbp_my_player_character))
  (AI|AIMoveTo self "0, 0, 0" _output_get 75.0 false))

(event EventBeginPlay)

(event Collision|EventActorBeginOverlap
  (params (OtherActor :type Actor%20Object%20Reference)))

(event EventTick
  (params (DeltaSeconds :type Float%20%28single-precision%29)))

(fn ConstructionScript)