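; Player character Blueprint that handles movement, item use and opening the inventory.
; Forward and right axis inputs move the character relative to the camera's yaw, and BeginPlay enables mouse click and hover events.
; Right-click traces WorldDynamic objects under the cursor and calls UseItem on inventory objects flagged IsNear.
; The I key creates the inventory widget and switches input to UI only; an older CheckInteraction chain is left unconnected.
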(event Collision|EventActorBeginOverlap
  (params (OtherActor :type Actor%20Object%20Reference)))

(event EventBeginPlay
  (bind _returnvalue (Game|GetPlayerController 0))
  (Variables|/Script/Engine.PlayerController|SetbEnableMouseOverEvents _returnvalue true)
  (Variables|/Script/Engine.PlayerController|SetbEnableClickEvents _returnvalue true))

(event Input|AxisEvents|InputAxisMoveForward
  (params (AxisValue :type Float%20%28single-precision%29))
  ;[1 1 1] Movement Handling
  (Pawn|Input|AddMovementInput (Math|Vector|GetForwardVector (Math|Rotator|MakeRotator 0.0 0.0 (.Yaw (Math|Rotator|BreakRotator (Transformation|GetWorldRotation (Variables|Default|GetCamera)))))) AxisValue false))

(event Input|AxisEvents|InputAxisMoveRight
  (params (AxisValue :type Float%20%28single-precision%29))
  ;[1 1 1] Movement Handling
  (Pawn|Input|AddMovementInput (Math|Vector|GetRightVector (Math|Rotator|MakeRotator 0.0 0.0 (.Yaw (Math|Rotator|BreakRotator (Transformation|GetWorldRotation (Variables|Default|GetCamera)))))) AxisValue false))

(event Input|MouseEvents|RightMouseButton
  (params (Key :type Key%20Structure :default "None"))
  (bind _returnvalue (Game|GetPlayerController 0))
  (bind _array (Utilities|Array|MakeArray "ObjectTypeQuery2"))
  (bind (_hitresult _returnvalue_2) (Class|PlayerController|GetHitResultUnderCursorforObjects _returnvalue _array true))
  (bind _hitactor (Collision|BreakHitResult _hitresult))
  ;[1 1 1] Interaction Handling
  (:Pressed
    (if _returnvalue_2
      (bind _asbp_inventory_objects (Utilities|Casting|CastToBP_InventoryObjects _hitactor))
      (if (Variables|/Game/Objects/BP_InventoryObjects.BP_InventoryObjects_C|GetIsNear _asbp_inventory_objects)
        (bind _asinteractable_objects (Utilities|Casting|CastToInteractableObjects _hitactor))
        (Class|PlayerCharacter|UseItem _asinteractable_objects)))))

(event Input|KeyboardEvents|I
  (params (Key :type Key%20Structure :default "None"))
  (bind _returnvalue (Game|GetPlayerController 0))
  (:Pressed
    (bind _returnvalue_2 (UserInterface|CreateWidget "/Game/Objects/InventoryWidget.InventoryWidget_C" _returnvalue))
    (UserInterface|Viewport|AddtoViewport _returnvalue_2 0)
    (Input|SetInputModeUIOnly _returnvalue _returnvalue_2 "DoNotLock" false)))

(fn ConstructionScript)